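; BP_Dummy is a test target actor for the Gameplay Ability System in Soulsbourne.
; On BeginPlay it listens for the Character.Damaged gameplay event and prints a debug message when one arrives.
; A ShowHealth event prints an attribute read from its AbilitySystemComponent.
; TakeDamage is an empty event, and an unconnected node would apply GE_30Damage to itself.
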(event Custom|ShowHealth
  (Development|PrintString (Utilities|String|ToString(Float) (.ReturnValue (Ability|Attribute|GetFloatAttributefromAbilitySystemComponent (Variables|Default|GetAbilitySystemComponent) "(AttributeName=\"Health\",Attribute=/Script/Soulsborne.SoulAttributeSet:Health,AttributeOwner=\"/Script/CoreUObject.Class'/Script/Soulsborne.SoulAttributeSet'\")")))))

(event Custom|TakeDamage)

(event EventBeginPlay
  (|CallParentFunction)
  (Ability|Async|WaitGameplayEventToActor 0 "(TagName=\"Character.Damaged\")"
    (:EventReceived
      (Development|PrintString "DAMAGE RECEIVED"))))

(event Collision|EventActorBeginOverlap
  (params (OtherActor :type Actor%20Object%20Reference))
  (|CallParentFunction OtherActor) ; This node is disabled and will not be called.\nDrag off pins to build functionality.
)

(event EventTick
  (params (DeltaSeconds :type Float%20%28single-precision%29))
  (|CallParentFunction DeltaSeconds) ; This node is disabled and will not be called.\nDrag off pins to build functionality.
)

(fn ConstructionScript
  (|CallParentFunction))