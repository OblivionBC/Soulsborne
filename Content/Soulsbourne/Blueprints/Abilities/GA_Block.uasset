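; Gameplay Ability that puts a Soulsbourne character into a blocking state.
; On activation it commits, applies the GE_IsBlocking effect to the owner and tells BP_SoulChar to start blocking.
; A tag-remove task ends the ability once Character.IsBlocking is removed.
; Ending calls FinishedBlocking on the character and cleans up the stored wait task.
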(event Ability|EventActivateAbility
  (Ability|CommitAbility)
  (Ability|ApplyGameplayEffectToOwner "/Game/Soulsbourne/Blueprints/Abilities/GE_IsBlocking.GE_IsBlocking_C")
  (bind _asbp_soul_char (Utilities|Casting|CastToBP_SoulChar (.OwnerActor (Utilities|Struct|BreakGameplayAbilityActorInfo (Ability|GetActorInfo)))))
  (Default|Blocking _asbp_soul_char)
  (bind _asynctaskproxy (Ability|Tasks|WaitGameplayTagRemove "(TagName=\"Character.IsBlocking\")" 0)
    (:then
      (Variables|Default|SetWaitForTagRemoval _asynctaskproxy))
    (:Removed
      (Ability|EndAbility))))

(event Ability|EventOnEndAbility
  (params (bWasCancelled :type Boolean))
  (bind _waitfortagremoval (Variables|Default|GetWaitForTagRemoval))
  (Default|FinishedBlocking (stale Ability|EventActivateAbility _asbp_soul_char))
  (Utilities|IsValid _waitfortagremoval
    (:Is%20Valid
      (GameplayTasks|EndTask _waitfortagremoval))))