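; Gameplay ability for the first greatsword attack, which commits and plays the attack montage.
; While it runs, a gameplay effect pauses stamina recharge, removed by granted tag when the ability ends.
; The ability ends when the montage completes, blends out or is interrupted.
; Disconnected leftover nodes would wait for a damage event to apply greatsword damage to a dummy target, but never execute.
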(event Ability|EventActivateAbility
  (Ability|CommitAbility)
  (Animation|Montage|PlayMontage (.SkeletalMeshComponent (Utilities|Struct|BreakGameplayAbilityActorInfo (Ability|GetActorInfo))) "/Game/Soulsbourne/Animations/Attacks/MONT_GreatswordAttack.MONT_GreatswordAttack"
    (:then
      (Ability|ApplyGameplayEffectToOwner "/Game/Soulsbourne/Blueprints/Abilities/Stamina/GE_PauseStamina.GE_PauseStamina_C"))
    (:OnCompleted
      (Ability|EndAbility :!label _label))
    (:OnBlendOut
      (goto _label))
    (:OnInterrupted
      (goto _label))))

(event Ability|EventOnEndAbility
  (params (bWasCancelled :type Boolean))
  (Ability|RemoveGameplayEffectFromOwnerWithGrantedTags "(GameplayTags=((TagName=\"Player.Attribute.Stamina.PauseRecharge\")))"))