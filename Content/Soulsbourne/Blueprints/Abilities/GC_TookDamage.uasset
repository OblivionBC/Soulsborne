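; GC_TookDamage is a gameplay cue that plays the damage reaction on BP_Dummy targets.
; On execute, it reads a float attribute from the dummy's ability system component to choose between a hit reaction and death.
; Above zero it plays the damage montage; otherwise it turns on mesh physics simulation for a ragdoll-style death, with debug prints marking damage and death.
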(fn OnExecute
  (params (MyTarget :type Actor%20Object%20Reference) (Parameters :type Gameplay%20Cue%20Parameters%20Structure%20%28by%20ref%29))
  (bind _asbp_dummy (Utilities|Casting|CastToBP_Dummy MyTarget))
  (Development|PrintString 0 "Damaged")
  (if (> (.ReturnValue (Ability|Attribute|GetFloatAttributefromAbilitySystemComponent (Variables|/Script/Soulsborne.SoulCharacter|GetAbilitySystemComponent _asbp_dummy) "(AttributeName=\"Health\",Attribute=/Script/Soulsborne.SoulAttributeSet:Health,AttributeOwner=\"/Script/CoreUObject.Class'/Script/Soulsborne.SoulAttributeSet'\")")) 0.0)
    (Animation|PlayAnimMontage _asbp_dummy "/Game/Soulsbourne/Animations/Hit/MONT_Damage.MONT_Damage" 1.0 "None")
    (return true)
    (else
      (Physics|SetSimulatePhysics (Variables|/Script/Engine.Character|GetMesh _asbp_dummy) true)
      (Development|PrintString 0 "dead"))))