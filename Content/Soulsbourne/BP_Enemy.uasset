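; Soulsbourne enemy Blueprint with a widget health bar and a sword attack driven by the Gameplay Ability System.
; On BeginPlay and every Tick it reads its health ratio through ProgressBarInterface and feeds it to the WBP_EnemyHealth bar.
; SwordAttack activates the AttackCombo ability by class on its Ability System Component.
; The OnDamaged event is empty, so the bar relies on polling.
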(event Collision|EventActorBeginOverlap
  (params (OtherActor :type Actor%20Object%20Reference)))

(event EventOnDamaged)

(event EventBeginPlay
  (bind _self self)
  (bind _aswbp_enemy_health (Utilities|Casting|CastToWBP_EnemyHealth (UserInterface|GetWidget (Variables|Default|GetWidget))))
  (if (Utilities|DoesObjectImplementInterface _self "/Script/Soulsborne.ProgressBarInterface")
    (bind _result (Class|ProgressBarInterface|GetHealthasRatio(Message) _self))
    (Default|Update (Variables|/Game/Soulsbourne/Blueprints/Widgets/WBP_EnemyHealth.WBP_EnemyHealth_C|GetEnemyHealthBar _aswbp_enemy_health) _result (Variables|/Game/Soulsbourne/Blueprints/Widgets/WBP_EnemyHealth.WBP_EnemyHealth_C|GetDeltaTime _aswbp_enemy_health))))

(event EventTick
  (params (DeltaSeconds :type Float%20%28single-precision%29))
  (bind _self self)
  (bind _aswbp_enemy_health (Utilities|Casting|CastToWBP_EnemyHealth (UserInterface|GetWidget (Variables|Default|GetWidget))))
  (if (Utilities|DoesObjectImplementInterface _self "/Script/Soulsborne.ProgressBarInterface")
    (bind _result (Class|ProgressBarInterface|GetHealthasRatio(Message) _self))
    (Default|Update (Variables|/Game/Soulsbourne/Blueprints/Widgets/WBP_EnemyHealth.WBP_EnemyHealth_C|GetEnemyHealthBar _aswbp_enemy_health) _result (Variables|/Game/Soulsbourne/Blueprints/Widgets/WBP_EnemyHealth.WBP_EnemyHealth_C|GetDeltaTime _aswbp_enemy_health))))

(fn ConstructionScript)

(fn SwordAttack
  (Abilities|TryActivateAbilitybyClass (Ability|GetAbilitySystemComponent 0) "/Script/Soulsborne.AttackCombo" true)
  (return 0.0))