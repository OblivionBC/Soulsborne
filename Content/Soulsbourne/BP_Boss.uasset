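; BP_Boss is a boss enemy that sets its max health on BeginPlay, then runs its parent's logic.
; BossAttack plays the boss attack montage and returns the result.
; A SphereTrace event traces for Pawns at the Slam component's location, ignoring its input locations, and only draws and prints the hit for debugging, with no damage applied.
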(event Custom|SphereTrace_1
  (params (StartLocation :type Vector) (EndLocation :type Vector))
  (bind _slam (Variables|Default|GetSlam))
  (bind _returnvalue (Transformation|GetWorldLocation _slam))
  (Development|PrintString "In it")
  (bind (_outhit _returnvalue_2) (Collision|SphereTraceForObjects _returnvalue _returnvalue 1e+02 (Utilities|Array|MakeArray "ObjectTypeQuery3") false 0 "ForDuration"))
  (Development|PrintString (Utilities|String|ToString(Boolean) _returnvalue_2))
  (Development|PrintString (Utilities|GetDisplayName (.HitActor (Collision|BreakHitResult _outhit)))))

(event EventBeginPlay
  (Class|BaseCharacter|SetMaxHealth 300)
  (|CallParentFunction))

(event Collision|EventActorBeginOverlap
  (params (OtherActor :type Actor%20Object%20Reference))
  (|CallParentFunction OtherActor) ; This node is disabled and will not be called.\nDrag off pins to build functionality.
)

(event EventTick
  (params (DeltaSeconds :type Float%20%28single-precision%29)))

(fn ConstructionScript
  (|CallParentFunction))

(fn BossAttack
  (bind _returnvalue (Animation|PlayAnimMontage "/Game/Soulsbourne/Animations/Attacks/MONT_BossAttack.MONT_BossAttack" 1.0 "None"))
  (return _returnvalue))